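; BP_Cube is a box the side-scroller character can push or pull.
; Overlapping its FWD component sets the character's CanInteractBox flag, without filtering the overlapping actor.
; While that and IsInteractingBox are true, Tick enables physics on SMCube and drives its velocity along its right vector from the negated movement axis scaled by character max speed.
; Debug prints remain, and an interpolated-location alternative sits unconnected.
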(event `self.ReceiveBeginPlay`
  ;[0.3305 0.2782 0.4792] Character Movement
  (bind _returnvalue (`GameplayStatics.GetActorOfClass` "/Game/SideScrollerBP/Blueprints/BP_SideScrollerCharacter.BP_SideScrollerCharacter_C"))
  (set `self.CharREF` _returnvalue))

(event `self.ReceiveTick`
  (params (DeltaSeconds :type "Float (single-precision)"))
  (bind _charref (`self.CharREF`))
  (bind _fwdbwdaxis (`/Game/SideScrollerBP/Blueprints/BP_SideScrollerCharacter.FwdBwdAxis` _charref))
  (bind _returnvalue (and (`/Game/SideScrollerBP/Blueprints/BP_SideScrollerCharacter.IsInteractingBox?` _charref) (`/Game/SideScrollerBP/Blueprints/BP_SideScrollerCharacter.CanInteractBox?` _charref)))
  (bind _returnvalue_2 (* _fwdbwdaxis (`MovementComponent.GetMaxSpeed` (`Character.CharacterMovement` _charref)) -1.0))
  ;[0.3305 0.2782 0.4792] Character Movement
  (`PrimitiveComponent.SetSimulatePhysics` (`self.SM_Cube`) _returnvalue)
  (if _returnvalue
    (`|ExecutionSequence`
      (:`then_0`
        (if (== _fwdbwdaxis 0.0)
          (`KismetSystemLibrary.PrintString` "player not moving forward" true true (struct :`R` 1.0 :`G` 0.023868 :`A` 1.0) 2.0 "24556")
          (elif (>= _fwdbwdaxis 0.0)
            (`KismetSystemLibrary.PrintString` "player moving forward" true true (struct :`R` 0.179489 :`G` 1.0 :`A` 1.0) 2.0 "5348")
            (`self.Speed/Direction` true _returnvalue_2)
            (else
              (`KismetSystemLibrary.PrintString` "player moving backward" true true (struct :`G` 0.784566 :`B` 1.0 :`A` 1.0) 2.0 "35645")
              (`self.Speed/Direction` true _returnvalue_2))))))))

(event `self.FWD.OnComponentBeginOverlap`
  (params (OverlappedComponent :type "PrimitiveComponent Object Reference") (OtherActor :type "Actor Object Reference") (OtherComp :type "PrimitiveComponent Object Reference") (OtherBodyIndex :type Integer) (bFromSweep :type Boolean) (SweepResult :type "HitResult Structure (by ref)"))
  ;[0.4646 1 0.5279] Overlap
  (set `/Game/SideScrollerBP/Blueprints/BP_SideScrollerCharacter.CanInteractBox?` true (`self.CharREF`))
  (`KismetSystemLibrary.PrintString` "Interact Box" true true (struct :`R` 1.0 :`G` 0.76695 :`A` 1.0) 2.0 "68468"))

(event `self.FWD.OnComponentEndOverlap`
  (params (OverlappedComponent :type "PrimitiveComponent Object Reference") (OtherActor :type "Actor Object Reference") (OtherComp :type "PrimitiveComponent Object Reference") (OtherBodyIndex :type Integer))
  ;[0.4646 1 0.5279] Overlap
  (set `/Game/SideScrollerBP/Blueprints/BP_SideScrollerCharacter.CanInteractBox?` false (`self.CharREF`))
  (`KismetSystemLibrary.PrintString` "Cannot Interact Box " true true (struct :`R` 0.306358 :`B` 1.0 :`A` 1.0) 2.0 "5464"))

(fn `UserConstructionScript`)